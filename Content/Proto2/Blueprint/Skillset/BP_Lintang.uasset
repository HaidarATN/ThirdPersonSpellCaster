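; BP_Lintang is the Lintang spell in the player's skillset, acting as an input-mode toggle with no effect logic of its own.
; ActivateSpell adds the IMC_Lintang Enhanced Input mapping context to the first player's controller.
; DeactivateSpell removes that context and clears ActivatedSpell on BP_MyCharacter.
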(event EventBeginPlay)

(event Collision|EventActorBeginOverlap
  (params (OtherActor :type Actor%20Object%20Reference)))

(event EventTick
  (params (DeltaSeconds :type Float%20%28single-precision%29)))

(event EventActivateSpell
  (bind _asplayer_controller (Utilities|Casting|CastToPlayerController (Pawn|GetController (Game|GetPlayerCharacter 0))))
  (Input|AddMappingContext (PlayerController|LocalPlayerSubsystems|GetEnhancedInputLocalPlayerSubsystem _asplayer_controller) "/Game/Proto2/Input/IMC_Lintang.IMC_Lintang" 0 (Utilities|Struct|MakeModifyContextOptions true false false)))

(event EventDeactivateSpell
  (bind _asplayer_controller (Utilities|Casting|CastToPlayerController (Pawn|GetController (Game|GetPlayerCharacter 0))))
  (Input|RemoveMappingContext (PlayerController|LocalPlayerSubsystems|GetEnhancedInputLocalPlayerSubsystem _asplayer_controller) "/Game/Proto2/Input/IMC_Lintang.IMC_Lintang" "(bIgnoreAllPressedKeysUntilRelease=True,bForceImmediately=False,bNotifyUserSettings=False)")
  (bind _asbp_my_character (Utilities|Casting|CastToBP_MyCharacter (Game|GetPlayerCharacter 0)))
  (Variables|/Game/Proto2/Blueprint/BP_MyCharacter.BP_MyCharacter_C|SetActivatedSpell _asbp_my_character 0))

(fn ConstructionScript)